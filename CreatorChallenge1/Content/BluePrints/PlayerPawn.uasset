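; PlayerPawn is a player-controlled pawn that moves by axis input and can dash into other PlayerPawns to knock them back.
; Axis input sets a normalized velocity, which Tick smooths by lerp to move the actor without sweep and face its travel direction.
; Dash briefly raises speed on the locally controlled pawn, but IsDashing is never cleared.
; Overlaps while dashing call the victim's ResetPos, costing a life and teleporting it to origin, or elsewhere when lives run out.
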(event Collision|EventActorBeginOverlap
  (params (OtherActor :type Actor%20Object%20Reference))
  (if (Variables|Default|GetisDashing)
    (bind _asplayer_pawn (Utilities|Casting|CastToPlayerPawn OtherActor))
    (CallFunction|ResetPos _asplayer_pawn)))

(event EventTick
  (params (DeltaSeconds :type Float%20%28single-precision%29))
  (bind _returnvalue (Transformation|GetActorLocation))
  (Variables|Default|SetActualVelocity (Math|Vector|Lerp(Vector) (Variables|Default|GetActualVelocity) (Variables|Default|GetVelocity) 0.1))
  (Transformation|SetActorLocation (+ _returnvalue (Variables|Default|GetActualVelocity)) false false)
  (Transformation|SetActorRotation (Math|Rotator|FindLookatRotation _returnvalue (+ _returnvalue (Variables|Default|GetActualVelocity)))))

(event Input|ActionEvents|InputActionDash
  (params (Key :type Key%20Structure :default "None"))
  (:Pressed
    (if (Pawn|IsLocallyControlled)
      (Variables|Default|SetisDashing true)
      (Variables|Default|Setplayer%20speed 5e+01)
      (Utilities|FlowControl|Delay 1.0)
      (Variables|Default|SetisDashing true)
      (Variables|Default|Setplayer%20speed 1e+01))))

(event Input|AxisEvents|InputAxisHorizontal
  (params (AxisValue :type Float%20%28single-precision%29))
  (Variables|Default|SetVelocity (* (Math|Vector|Normalize (+ (* "0.000000,1.000000,0.000000" (stale Input|AxisEvents|InputAxisVertical AxisValue)) (* "-1.000000,0.000000,0.000000" AxisValue))) (Variables|Default|Getplayer%20speed))))

(event Input|AxisEvents|InputAxisVertical
  (params (AxisValue :type Float%20%28single-precision%29))
  (Variables|Default|SetVelocity (* (Math|Vector|Normalize (+ (* "0.000000,1.000000,0.000000" AxisValue) (* "-1.000000,0.000000,0.000000" (stale Input|AxisEvents|InputAxisHorizontal AxisValue)))) (Variables|Default|Getplayer%20speed))))

(fn ConstructionScript)

(fn ResetPos
  (Variables|Default|SetLives (- (Variables|Default|GetLives) 1))
  (if (<= (Variables|Default|GetLives) 0)
    (Transformation|SetActorLocation "100.000000,100.000000,100.000000" false false)
    (else
      (Transformation|SetActorLocation "0, 0, 0" false false))))